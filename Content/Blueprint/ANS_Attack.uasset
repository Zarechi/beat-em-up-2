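; Anim notify state "Attack" that opens a melee damage window on BP_Player's animations.
; Each tick it box-traces for Pawns in place at the WeaponHandler socket, oriented to it and skipping actors in the player's HittedActors.
; The hit actor is added to that list and takes the player's Damage, limiting each target to one hit per window.
; Notify end clears the list.
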(fn `GetNotifyName`
  (returns (ReturnValue :type String))
  (return "Attack"))

(fn `Received_NotifyEnd`
  (params (MeshComp :type "SkeletalMeshComponent Object Reference") (Animation :type "AnimSequenceBase Object Reference"))
  (returns (ReturnValue :type Boolean))
  (`KismetArrayLibrary.Array_Clear` (`/Game/Blueprint/Characters/Player/BP_Player.HittedActors` (cast `/Game/Blueprint/Characters/Player/BP_Player` (`ActorComponent.GetOwner` MeshComp) :!pure true)))
  (return false))

(fn `Received_NotifyTick`
  (params (MeshComp :type "SkeletalMeshComponent Object Reference") (Animation :type "AnimSequenceBase Object Reference") (FrameDeltaTime :type "Float (double-precision)"))
  (returns (ReturnValue :type Boolean))
  (locals (Player :type "/Game/Blueprint/Characters/Player/BP_Player Object Reference"))
  (bind _meshcomp (`local.MeshComp`))
  (bind _returnvalue (`SceneComponent.GetSocketLocation` _meshcomp "WeaponHandler"))
  (set `local.Player` (cast `/Game/Blueprint/Characters/Player/BP_Player` (`ActorComponent.GetOwner` (`local.MeshComp`)) :!pure true))
  (bind _outhit (`KismetSystemLibrary.BoxTraceSingleForObjects` _meshcomp _returnvalue _returnvalue (`self.WeaponHalfSize`) (`SceneComponent.GetSocketRotation` _meshcomp "WeaponHandler") (`|MakeArray` "ObjectTypeQuery3" :!type "EObjectTypeQuery Enum") false (`/Game/Blueprint/Characters/Player/BP_Player.HittedActors` (`local.Player`)) (`self.Draw Debug Type`)))
  (bind (_bblockinghit _binitialoverlap _time _distance _location _impactpoint _normal _impactnormal _physmat _hitactor) (`GameplayStatics.BreakHitResult` _outhit))
  (`KismetArrayLibrary.Array_AddUnique` (`/Game/Blueprint/Characters/Player/BP_Player.HittedActors` (`local.Player`)) _hitactor)
  (`GameplayStatics.ApplyDamage` _hitactor (`/Game/Blueprint/Characters/BP_BaseCharacter.Damage` (`local.Player`)))
  (return false))