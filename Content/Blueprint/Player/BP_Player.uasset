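; Player character Blueprint with walk, sprint, jump, mouse look and an axe attack.
; Input moves along actor axes, swaps max walk speed for sprint, turns by controller yaw and pitches only the SpringArm.
; Attack plays an Axe_Combo1 montage section chosen by a counter, blocked while IsAttacking; montage completion resets both.
; Incoming damage subtracts from HP, which prints on screen every tick, with no death handling.
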(event `self.ReceiveBeginPlay`
  (set `CharacterMovementComponent.MaxWalkSpeed` (`self.MaxWalkSpeed`) (`self.CharacterMovement`)))

(event `self.ReceiveAnyDamage`
  (params (Damage :type "Float (single-precision)") (DamageType :type "DamageType Object Reference") (InstigatedBy :type "Controller Object Reference") (DamageCauser :type "Actor Object Reference"))
  (set `self.HP` (- (`self.HP`) Damage)))

(event `self.ReceiveTick`
  (params (DeltaSeconds :type "Float (single-precision)"))
  (`KismetSystemLibrary.PrintString` (`KismetStringLibrary.Concat_StrStr` (`KismetSystemLibrary.GetDisplayName` self) " = " (`KismetStringLibrary.Conv_DoubleToString` (`self.HP`))) true true (struct :`G` 0.66 :`B` 1.0 :`A` 1.0) DeltaSeconds))

(event `InputAxis|MoveForward`
  (params (AxisValue :type "Float (single-precision)"))
  (`self.AddMovementInput` (`self.GetActorForwardVector`) AxisValue))

(event `InputAxis|MoveRight`
  (params (AxisValue :type "Float (single-precision)"))
  (`self.AddMovementInput` (`self.GetActorRightVector`) AxisValue))

(event `InputAction|Run`
  (params (Key :type "Key Structure"))
  (:`Pressed`
    (set `CharacterMovementComponent.MaxWalkSpeed` (`self.MaxSprintSpeed`) (`self.CharacterMovement`)))
  (:`Released`
    (set `CharacterMovementComponent.MaxWalkSpeed` (`self.MaxWalkSpeed`) (`self.CharacterMovement`))))

(event `InputAxis|Turn`
  (params (AxisValue :type "Float (single-precision)"))
  (`self.AddControllerYawInput` (* AxisValue (`self.MouseSensibiltyX`))))

(event `InputAxis|LookUp`
  (params (AxisValue :type "Float (single-precision)"))
  (`SceneComponent.K2_AddLocalRotation` (`self.SpringArm`) (`KismetMathLibrary.MakeRotator` 0.0 (* AxisValue (`self.MouseSensibiltyY`))) false false))

(event `InputAction|Attack`
  (params (Key :type "Key Structure"))
  (:`Pressed`
    (if (not (`self.IsAttacking?`))
      (`|PlayMontage` (`self.Mesh`) "/Game/Animation/Attack/Axe_Combo1_Montage.Axe_Combo1_Montage" 1.0 0.0 (select `int` (`self.AttackCpt`) :`0` "01" :`1` "02" :`2` "03" :!type "Name")
        (:`then`
          (set `self.IsAttacking?` true)
          (`/Engine/EditorBlueprintResources/StandardMacros.IncrementInt` (`self.AttackCpt`)))
        (:`OnCompleted`
          (set `self.IsAttacking?` false) ; Combo finished
          (set `self.AttackCpt` 0))))))

(event `InputAction|Jump`
  (params (Key :type "Key Structure"))
  (:`Pressed`
    (`self.Jump`)))

(fn `UserConstructionScript`)