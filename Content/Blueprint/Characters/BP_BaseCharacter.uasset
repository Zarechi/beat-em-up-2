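; Base character Blueprint with a simple hit point pool and configurable walk speed.
; On BeginPlay it copies MaxWalkSpeed to the movement component, and AnyDamage subtracts incoming damage from HP with no clamp or death handling.
; Tick prints the character's display name and current HP to the screen every frame as a debug readout.
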(event `self.ReceiveBeginPlay`
  (set `CharacterMovementComponent.MaxWalkSpeed` (`self.MaxWalkSpeed`) (`self.CharacterMovement`)))

(event `self.ReceiveTick`
  (params (DeltaSeconds :type "Float (single-precision)"))
  (`KismetSystemLibrary.PrintString` (`KismetStringLibrary.Concat_StrStr` (`KismetSystemLibrary.GetDisplayName` self) " = " (`KismetStringLibrary.Conv_DoubleToString` (`self.HP`))) true true (struct :`G` 0.66 :`B` 1.0 :`A` 1.0) DeltaSeconds))

(event `self.ReceiveAnyDamage`
  (params (Damage :type "Float (single-precision)") (DamageType :type "DamageType Object Reference") (InstigatedBy :type "Controller Object Reference") (DamageCauser :type "Actor Object Reference"))
  (set `self.HP` (- (`self.HP`) Damage)))

(fn `UserConstructionScript`)