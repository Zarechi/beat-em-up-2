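; Player character Blueprint that maps input to movement, sprint, jump, mouse look and axe attacks.
; Turn input yaws the controller, while LookUp pitches the spring arm locally, both scaled by per-axis sensitivity.
; Run swaps max walk speed between sprint and walk values.
; Grounded attacks, gated by IsAttacking, play a combo montage section chosen by a counter, with both reset on montage completion.
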(event `InputAxis|MoveForward`
  (params (AxisValue :type "Float (single-precision)"))
  (`self.AddMovementInput` (`self.GetActorForwardVector`) AxisValue))

(event `InputAxis|MoveRight`
  (params (AxisValue :type "Float (single-precision)"))
  (`self.AddMovementInput` (`self.GetActorRightVector`) AxisValue))

(event `InputAction|Run`
  (params (Key :type "Key Structure"))
  (:`Pressed`
    (set `CharacterMovementComponent.MaxWalkSpeed` (`self.MaxSprintSpeed`) (`self.CharacterMovement`)))
  (:`Released`
    (set `CharacterMovementComponent.MaxWalkSpeed` (`self.MaxWalkSpeed`) (`self.CharacterMovement`))))

(event `InputAxis|Turn`
  (params (AxisValue :type "Float (single-precision)"))
  (`self.AddControllerYawInput` (* AxisValue (`self.MouseSensibiltyX`))))

(event `InputAxis|LookUp`
  (params (AxisValue :type "Float (single-precision)"))
  (`SceneComponent.K2_AddLocalRotation` (`self.SpringArm`) (`KismetMathLibrary.MakeRotator` 0.0 (* AxisValue (`self.MouseSensibiltyY`))) false false))

(event `InputAction|Attack`
  (params (Key :type "Key Structure"))
  (:`Pressed`
    (if (and (not (`self.IsAttacking?`)) (not (`NavMovementComponent.IsFalling` (`self.CharacterMovement`))))
      (`|PlayMontage` (`self.Mesh`) "/Game/Animation/Attack/Axe_Combo1_Montage.Axe_Combo1_Montage" 1.0 0.0 (select `int` (`self.AttackCpt`) :`0` "01" :`1` "02" :`2` "03" :!type "Name")
        (:`then`
          (set `self.IsAttacking?` true)
          (`/Engine/EditorBlueprintResources/StandardMacros.IncrementInt` (`self.AttackCpt`)))
        (:`OnCompleted`
          (set `self.IsAttacking?` false) ; Combo finished
          (set `self.AttackCpt` 0))))))

(event `InputAction|Jump`
  (params (Key :type "Key Structure"))
  (:`Pressed`
    (`self.Jump`)))

(fn `UserConstructionScript`)